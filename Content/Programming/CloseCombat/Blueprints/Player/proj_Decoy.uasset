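; Thrown decoy ball projectile that asks the player pawn to spawn a decoy when it hits the floor, with a half-second lifespan.
; Sphere1's overlap prints a debug string, matches the floor by a hard-coded component display name, then calls SpawnDecoyFromThrownBall on the first Pawn_CloseCombat found.
; A timeline-driven movement graph and a QuitGame node are disconnected, and the Tick visibility check does nothing.
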(event OnComponentBeginOverlap(Sphere1)
  (params (OverlappedComponent :type Primitive%20Component%20Object%20Reference) (OtherActor :type Actor%20Object%20Reference) (OtherComp :type Primitive%20Component%20Object%20Reference) (OtherBodyIndex :type Integer) (bFromSweep :type Boolean) (SweepResult :type Hit%20Result%20Structure%20%28by%20ref%29))
  (Development|PrintString "Hello")
  (if (Utilities|Enum|Equal(Enum) (Utilities|GetDisplayName OtherComp) "Floor.StaticMeshComponent0 SM_Template_Map_Floor")
    (bind _outactors (Actor|GetAllActorsOfClass "/Game/Programming/CloseCombat/Blueprints/Player/Pawn_CloseCombat.Pawn_CloseCombat_C"))
    (Default|SpawnDecoyfromThrownBall (Utilities|Array|Get(acopy) _outactors))))

(event EventBeginPlay
  (Actor|SetLifeSpan 0.5))

(event EventTick
  (params (DeltaSeconds :type Float%20%28single-precision%29))
  (if (Rendering|IsVisible (Variables|Default|GetSphere))
    _))

(fn ConstructionScript)